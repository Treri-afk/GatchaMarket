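; Base item actor that signals the player's hotbar component when the first-person character is within pickup range.
; On sphere overlap it caches the character, flags an item as close and passes itself to the hotbar.
; Any end overlap clears only the close flag through the cached reference, without checking which actor left.
; UseItem receives a hotbar reference but only prints a placeholder string.
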(event `self.Sphere.OnComponentBeginOverlap`
  (params (OverlappedComponent :type "PrimitiveComponent Object Reference") (OtherActor :type "Actor Object Reference") (OtherComp :type "PrimitiveComponent Object Reference") (OtherBodyIndex :type Integer) (bFromSweep :type Boolean) (SweepResult :type "HitResult Structure (by ref)"))
  (bind _asbp_first_person_character (cast `/Game/FirstPerson/Blueprints/BP_FirstPersonCharacter` OtherActor))
  (set `self.PlayerRef` _asbp_first_person_character)
  (bind _bpc_hotbar (`/Game/FirstPerson/Blueprints/BP_FirstPersonCharacter.BPC_HotBar` _asbp_first_person_character))
  (set `/Game/FirstPerson/Blueprints/Component/BPC_HotBar.ItemClose` true _bpc_hotbar)
  (set `/Game/FirstPerson/Blueprints/Component/BPC_HotBar.Item` self _bpc_hotbar))

(event `self.Sphere.OnComponentEndOverlap`
  (params (OverlappedComponent :type "PrimitiveComponent Object Reference") (OtherActor :type "Actor Object Reference") (OtherComp :type "PrimitiveComponent Object Reference") (OtherBodyIndex :type Integer))
  (set `/Game/FirstPerson/Blueprints/Component/BPC_HotBar.ItemClose` false (`/Game/FirstPerson/Blueprints/BP_FirstPersonCharacter.BPC_HotBar` (`self.PlayerRef`))))

(fn `UseItem`
  (params (HotBarRef :type "/Game/FirstPerson/Blueprints/Component/BPC_HotBar Object Reference"))
  (`KismetSystemLibrary.PrintString` "Hello"))

(fn `UserConstructionScript`)